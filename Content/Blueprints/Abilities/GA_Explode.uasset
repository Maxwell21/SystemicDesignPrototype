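; Gameplay ability that makes its avatar explode after a delayed spark fuse, cancelled if the Stimulus.Fire tag is removed first.
; On activation it adds the FireSparks cue and removes the Burn cue shortly afterwards.
; When the fuse ends, it spawns GC_Explosion and sphere-traces the Visibility channel with debug drawing, dealing massive damage to hit actors.
; The avatar is destroyed when the ability ends without cancellation.
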(event Ability|EventActivateAbility
  (bind _returnvalue (Ability|GetAvatarActorfromActorInfo))
  (bind _returnvalue_2 (Transformation|GetActorLocation _returnvalue))
  (Ability|Tasks|WaitGameplayTagRemove "(TagName=\"Stimulus.Fire\")" 0 true
    (:then
      (Utilities|FlowControl|Sequence
        (:then_0
          (GameplayCue|AddGameplayCue :GameplayCueTag "(TagName=\"GameplayCue.FireSparks\")")
          (Ability|Tasks|WaitDelay (Variables|Default|GetDelayBeforeExplode)
            (:OnFinish
              (GameplayCue|RemoveGameplayCue "(TagName=\"GameplayCue.FireSparks\")")
              (Game|SpawnActorfromClass "/Game/Blueprints/Cues/GC_Explosion.GC_Explosion_C" (Math|Transform|MakeTransform _returnvalue_2 "0, 0, 0" "1.000000,1.000000,1.000000") "Undefined" 0 0)
              (bind _outhits (Collision|MultiSphereTraceByChannel _returnvalue_2 _returnvalue_2 (Variables|Default|GetRadius) "TraceTypeQuery1" false 0 "ForDuration"))
              (for _array_element _outhits
                (Game|Damage|ApplyDamage (.HitActor (Collision|BreakHitResult _array_element)) 555555.0 0 0))
              (Ability|EndAbility))))
        (:then_1
          (Ability|Tasks|WaitDelay 0.7
            (:OnFinish
              (GameplayCue|RemoveGameplayCue "(TagName=\"GameplayCue.Burn\")"))))))
    (:Removed
      (Ability|CancelAbility))))

(event Ability|EventOnEndAbility
  (params (bWasCancelled :type Boolean))
  (if (not bWasCancelled)
    (Actor|DestroyActor (Ability|GetAvatarActorfromActorInfo))))