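; EntitySystemComponent is a component that answers stimulus queries for its owning entity, with stimuli tied to Gameplay Ability System effects.
; HasStimulus checks whether a given item is in the StimulusEffects collection.
; GetActiveStimulusEffects queries the owner's Ability System Component for active effects matching each owned gameplay tag and returns their unique classes, without filtering against StimulusEffects.
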(fn HasStimulus
  (params (Item :type Gameplay%20Effect%20Class%20Reference%20%28by%20ref%29))
  (return (Utilities|Array|ContainsItem (Variables|Default|GetStimulusEffects) Item)))

(fn GetActiveStimulusEffects
  (bind _returnvalue (Components|GetOwner))
  (bind _returnvalue_2 (Ability|GetAbilitySystemComponent _returnvalue))
  (Utilities|IsValid _returnvalue_2
    (:Is%20Valid
      (for _array_element (GameplayTags|BreakGameplayTagContainer (GameplayTags|GetOwnedGameplayTags _returnvalue_2 :!class /Script/GameplayTags.GameplayTagAssetInterface))
        (bind _returnvalue_3 (GameplayEffects|GetActiveEffectswithAllTags _returnvalue_2 (GameplayTags|MakeGameplayTagContainerfromTag _array_element)))
        (for _array_element_2 _returnvalue_3
          (Utilities|Array|AddUnique (LocalVariables|GetLocalEffects) (Utilities|GetClass (Ability|GameplayEffect|GetGameplayEffectfromActiveEffectHandle _array_element_2)))))
      (return (LocalVariables|GetLocalEffects)))))